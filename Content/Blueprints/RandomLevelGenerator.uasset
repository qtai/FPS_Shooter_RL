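; Actor that builds a random tiled level at BeginPlay from a list of streaming sublevels.
; It loops over a NumX by NumY grid and, per cell, creates a uniquely named instance of a randomly picked level from LevelNames.
; Each instance is offset by LevelSize so the grid is centred on the world origin, then set to load and become visible.
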(event `self.ReceiveBeginPlay`
  (bind _levelnames (`self.LevelNames`))
  (for _index (range (`self.NumX`))
    (set `self.LoopX` _index)
    (for _index_2 (range (`self.NumY`))
      (set `self.LoopY` _index_2)
      (bind _returnvalue (`LevelStreaming.CreateInstance` (`GameplayStatics.GetStreamingLevel` (`|GetArrayItem` _levelnames (`KismetMathLibrary.RandomIntegerInRange` 0 (`KismetArrayLibrary.Array_LastIndex` _levelnames)))) (`KismetStringLibrary.Concat_StrStr` (`KismetStringLibrary.Conv_IntToString` (`self.LoopX`)) "x" (`KismetStringLibrary.Conv_IntToString` (`self.LoopY`)))))
      (set `LevelStreaming.LevelTransform` (`KismetMathLibrary.MakeTransform` (`KismetMathLibrary.MakeVector` (+ (- (* (`self.LoopX`) (`self.LevelSize`)) (/ (* (`self.NumX`) (`self.LevelSize`)) 2.0)) (/ (`self.LevelSize`) 2.0)) (+ (- (* (`self.LoopY`) (`self.LevelSize`)) (/ (* (`self.NumY`) (`self.LevelSize`)) 2.0)) (/ (`self.LevelSize`) 2.0)))) _returnvalue)
      (set `LevelStreaming.bShouldBeLoaded` true _returnvalue)
      (set `LevelStreaming.bShouldBeVisible` true _returnvalue))))

(fn `UserConstructionScript`)