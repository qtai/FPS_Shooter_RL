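; BP_GridGenTest is a test actor that spawns a two-dimensional grid of actors around its own location at BeginPlay.
; Nested loops over NumPartsX and NumPartsY place one actor per cell, spaced by GridSize plus per-axis padding.
; Each position is shifted back by half the unpadded grid extent, so padding is not included in the centering.
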(event `self.ReceiveBeginPlay`
  (for _index (range (`self.NumPartsX`))
    (for _index_2 (range (`self.NumPartsY`))
      (`|SpawnActorFromClass` "/Game/Blueprints/test/BP_TestMeshForGen.BP_TestMeshForGen_C" (`KismetMathLibrary.MakeTransform` (`KismetMathLibrary.MakeVector` (- (+ (* _index (+ (`self.GridSize`) (`self.PaddingX`))) (.x (`self.K2_GetActorLocation`))) (/ (* (`self.NumPartsX`) (`self.GridSize`)) 2.0)) (- (+ (* _index_2 (+ (`self.GridSize`) (`self.PaddingY`))) (.y (`self.K2_GetActorLocation`))) (/ (* (`self.NumPartsY`) (`self.GridSize`)) 2.0)))) "Undefined" "OverrideRootScale" null null))))

(fn `UserConstructionScript`)